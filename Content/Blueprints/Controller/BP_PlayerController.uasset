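; Player controller for an FPS mission that starts with input disabled and handles escape, quest toggle and pause.
; Pressing E checks objectives in order: drones cleared, battery core destroyed, Voron eliminated, at the escape vehicle with the key.
; Unmet steps post an announcement through FPSGameMode, while meeting all updates the quest and triggers the win.
; Enhanced Input actions forward quest-widget toggling to the HUD and pausing to the game mode.
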(event Input|EnhancedActionEvents|EnhancedInputActionIA_ToggleQuest
  (params (ActionValue :type Boolean) (ElapsedSeconds :type Float%20%28double-precision%29) (TriggeredSeconds :type Float%20%28double-precision%29) (InputAction :type Input%20Action%20Object%20Reference :default "/Game/Input/Actions/IA_ToggleQuest.IA_ToggleQuest"))
  (:Started
    (bind _asfpsgame_mode (Utilities|Casting|CastToFPSGameMode (Game|GetGameMode)))
    (Default|ToggleQuestWidget (Variables|/Game/Blueprints/Game/FPSGameMode.FPSGameMode_C|GetHUD _asfpsgame_mode))))

(event Input|EnhancedActionEvents|EnhancedInputActionIA_Pause
  (params (ActionValue :type Boolean) (ElapsedSeconds :type Float%20%28double-precision%29) (TriggeredSeconds :type Float%20%28double-precision%29) (InputAction :type Input%20Action%20Object%20Reference :default "/Game/Input/Actions/IA_Pause.IA_Pause"))
  (:Started
    (bind _asfpsgame_mode (Utilities|Casting|CastToFPSGameMode (Game|GetGameMode)))
    (Default|PauseGame _asfpsgame_mode)))

(event EventBeginPlay
  (|CallParentFunction)
  (Input|DisableInput self))

(event EventTick
  (params (DeltaSeconds :type Float%20%28single-precision%29)))

(event Input|KeyboardEvents|E
  (params (Key :type Key%20Structure :default "None"))
  (:Pressed
    (bind _asbp_player (Utilities|Casting|CastToBP_Player (Game|GetPlayerCharacter 0)))
    (bind _asfpsgame_mode (Utilities|Casting|CastToFPSGameMode (Game|GetGameMode)))
    (if (<= (Variables|/Game/Blueprints/Game/FPSGameMode.FPSGameMode_C|GetNoOfDrones _asfpsgame_mode) 0)
      (bind _returnvalue (Actor|GetActorOfClass "/Game/Blueprints/Props/BP_Core.BP_Core_C"))
      (Utilities|IsValid _returnvalue
        (:Is%20Valid
          (Default|UpdateAnnouncement _asfpsgame_mode "Find and Destroy Drone Battery Core"))
        (:Is%20Not%20Valid
          (bind _returnvalue_2 (Actor|GetActorOfClass "/Game/Blueprints/Character/V2/Boss/BP_Boss.BP_Boss_C"))
          (Utilities|IsValid _returnvalue_2
            (:Is%20Valid
              (Default|UpdateAnnouncement _asfpsgame_mode "Voron Must Be Eliminated"))
            (:Is%20Not%20Valid
              (if (Variables|/Script/BrotherhoodFPS.BH_CharacterPlayer|GetbIsAtEscapeVehicle _asbp_player)
                (if (Variables|/Script/BrotherhoodFPS.BH_CharacterPlayer|GetbHasKey _asbp_player)
                  (Default|UpdateQuest _asfpsgame_mode (Utilities|String|MakeLiteralString "Escape With Voron's Vehicle"))
                  (Default|PlayerWon _asfpsgame_mode)
                  (else
                    (Default|UpdateAnnouncement _asfpsgame_mode "Key Needed To Start Vehicle")))
                (else
                  (Default|UpdateAnnouncement _asfpsgame_mode "Find Escape Vehicle")))))))
      (else
        (Default|UpdateAnnouncement _asfpsgame_mode "Clear Zone Before you bail out soldier")))))

(fn ConstructionScript)
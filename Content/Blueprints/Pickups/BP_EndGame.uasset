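; BP_EndGame is the escape vehicle trigger that marks where the player can end the game.
; Entering its sphere sets IsAtEscapeVehicle on BP_Player, and leaving clears it.
; On entry it checks HasKey: with the key, FPSGameMode shows a press-E escape tutorial prompt.
; Without it, the game mode announces that a key is needed and a no-key sound plays.
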(event OnComponentBeginOverlap(Sphere)
  (params (OverlappedComponent :type Primitive%20Component%20Object%20Reference) (OtherActor :type Actor%20Object%20Reference) (OtherComp :type Primitive%20Component%20Object%20Reference) (OtherBodyIndex :type Integer) (bFromSweep :type Boolean) (SweepResult :type Hit%20Result%20Structure%20%28by%20ref%29))
  (bind _asbp_player (Utilities|Casting|CastToBP_Player OtherActor))
  (Variables|/Script/BrotherhoodFPS.BH_CharacterPlayer|SetbIsAtEscapeVehicle _asbp_player true)
  (if (Variables|/Script/BrotherhoodFPS.BH_CharacterPlayer|GetbHasKey _asbp_player)
    (bind _asfpsgame_mode (Utilities|Casting|CastToFPSGameMode (Game|GetGameMode)))
    (Default|UpdateTutorial _asfpsgame_mode "Press" "To Escape in Vehicle" "/Game/Assets/UI/Inputs/keyboard_e.keyboard_e")
    (else
      (bind _asfpsgame_mode_2 (Utilities|Casting|CastToFPSGameMode (Game|GetGameMode)))
      (Default|UpdateAnnouncement _asfpsgame_mode_2 "Find Key To Start This Vehicle")
      (Audio|PlaySound2D "/Game/Assets/Sounds/Voice/DroneDefiance-TruckHasNoKey_Cue.DroneDefiance-TruckHasNoKey_Cue" 1.0 1.0 0.0 0 0))))

(event OnComponentEndOverlap(Sphere)
  (params (OverlappedComponent :type Primitive%20Component%20Object%20Reference) (OtherActor :type Actor%20Object%20Reference) (OtherComp :type Primitive%20Component%20Object%20Reference) (OtherBodyIndex :type Integer))
  (bind _asbp_player (Utilities|Casting|CastToBP_Player OtherActor))
  (Variables|/Script/BrotherhoodFPS.BH_CharacterPlayer|SetbIsAtEscapeVehicle _asbp_player false))

(event EventBeginPlay)

(event Collision|EventActorBeginOverlap
  (params (OtherActor :type Actor%20Object%20Reference)))

(event EventTick
  (params (DeltaSeconds :type Float%20%28single-precision%29)))

(fn ConstructionScript
  (|CallParentFunction))
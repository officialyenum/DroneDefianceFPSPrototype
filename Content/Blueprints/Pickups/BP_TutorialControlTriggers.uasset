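; BP_TutorialControlTriggers is a placeable trigger volume that shows a control tutorial when the player walks into it.
; When BP_Player overlaps its Box, it passes its TutorialText, ActionType and ButtonImage to FPSGameMode's UpdateTutorial.
; It then destroys itself, so each trigger fires only once.
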(event OnComponentBeginOverlap(Box)
  (params (OverlappedComponent :type Primitive%20Component%20Object%20Reference) (OtherActor :type Actor%20Object%20Reference) (OtherComp :type Primitive%20Component%20Object%20Reference) (OtherBodyIndex :type Integer) (bFromSweep :type Boolean) (SweepResult :type Hit%20Result%20Structure%20%28by%20ref%29))
  (Utilities|Casting|CastToBP_Player OtherActor)
  (bind _asfpsgame_mode (Utilities|Casting|CastToFPSGameMode (Game|GetGameMode)))
  (Default|UpdateTutorial _asfpsgame_mode (Variables|Default|GetTutorialText) (Variables|Default|GetActionType) (Variables|Default|GetButtonImage))
  (Actor|DestroyActor))

(event EventBeginPlay
  (|CallParentFunction) ; This node is disabled and will not be called.\nDrag off pins to build functionality.
)

(fn ConstructionScript
  (|CallParentFunction))
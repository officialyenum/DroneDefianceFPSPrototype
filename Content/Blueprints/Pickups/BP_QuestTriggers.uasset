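; BP_QuestTriggers is a one-shot trigger volume that announces a quest message when the player walks into it.
; On Box overlap by BP_Player, it sends QuestText in a red tint to FPSGameMode's announcement and plays the VoiceToPlay sound in 2D.
; It destroys itself after a short delay.
; The PerformAction event only casts the game mode and has no further effect.
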(event OnComponentBeginOverlap(Box)
  (params (OverlappedComponent :type Primitive%20Component%20Object%20Reference) (OtherActor :type Actor%20Object%20Reference) (OtherComp :type Primitive%20Component%20Object%20Reference) (OtherBodyIndex :type Integer) (bFromSweep :type Boolean) (SweepResult :type Hit%20Result%20Structure%20%28by%20ref%29))
  (Utilities|Casting|CastToBP_Player OtherActor)
  (bind _asfpsgame_mode (Utilities|Casting|CastToFPSGameMode (Game|GetGameMode)))
  (Default|UpdateAnnouncement _asfpsgame_mode (Variables|Default|GetQuestText) "(R=1.000000,G=0.043458,B=0.000000,A=1.000000)")
  (Audio|PlaySound2D (Variables|Default|GetVoiceToPlay) 1.0 1.0 0.0 0 0)
  (Utilities|FlowControl|Delay 0.2)
  (Actor|DestroyActor))

(event Custom|PerformAction
  (Utilities|Casting|CastToFPSGameMode (Game|GetGameMode)))

(event EventBeginPlay
  (|CallParentFunction) ; This node is disabled and will not be called.\nDrag off pins to build functionality.
)

(event Collision|EventActorBeginOverlap
  (params (OtherActor :type Actor%20Object%20Reference))
  (|CallParentFunction OtherActor) ; This node is disabled and will not be called.\nDrag off pins to build functionality.
)

(event EventTick
  (params (DeltaSeconds :type Float%20%28single-precision%29))
  (|CallParentFunction DeltaSeconds) ; This node is disabled and will not be called.\nDrag off pins to build functionality.
)

(fn ConstructionScript
  (|CallParentFunction))
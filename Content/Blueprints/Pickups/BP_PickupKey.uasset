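; BP_PickupKey is a pickup actor for the escape vehicle key.
; When a BP_Player overlaps its sphere, it plays a pickup sound and sets the player's HasKey flag.
; It then updates the key quest and shows a green acquisition announcement through FPSGameMode, plays a second sound cue and destroys itself.
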(event OnComponentBeginOverlap(Sphere)
  (params (OverlappedComponent :type Primitive%20Component%20Object%20Reference) (OtherActor :type Actor%20Object%20Reference) (OtherComp :type Primitive%20Component%20Object%20Reference) (OtherBodyIndex :type Integer) (bFromSweep :type Boolean) (SweepResult :type Hit%20Result%20Structure%20%28by%20ref%29))
  (bind _asbp_player (Utilities|Casting|CastToBP_Player OtherActor))
  (Audio|PlaySound2D (Variables|Default|GetPickupSound) 1.0 1.0 0.0 0 0)
  (Variables|/Script/BrotherhoodFPS.BH_CharacterPlayer|SetbHasKey _asbp_player true)
  (bind _asfpsgame_mode (Utilities|Casting|CastToFPSGameMode (Game|GetGameMode)))
  (Default|UpdateQuest _asfpsgame_mode (Utilities|String|MakeLiteralString "Find Escape Vehicle Key"))
  (Default|UpdateAnnouncement _asfpsgame_mode "Escape Vehicle Key Acquired" "(R=0.000000,G=1.000000,B=0.106813,A=1.000000)")
  (Audio|PlaySound2D "/Game/Assets/Sounds/Voice/DroneDefiance-FindKey_Cue.DroneDefiance-FindKey_Cue" 1.0 1.0 0.0 0 0)
  (Actor|DestroyActor))

(fn ConstructionScript)
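; BP_Player is the first-person player character, handling health feedback, death and head bob.
; Damage checks update the HUD through FPSGameMode, play a hit animation and camera shake, and report death when health runs out.
; Shot and hit stats are forwarded to the game mode.
; Tick picks sprint, walk or idle shakes from AnimBP state unless aiming, and construction snaps the gun to the GripPoint socket.
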(event Custom|UpdateBloodAnimation
  (bind _as_fpsgame_mode (Variables|Default|GetAs%20FPSGame%20Mode))
  (bind _hud (Variables|/Game/Blueprints/Game/FPSGameMode.FPSGameMode_C|GetHUD _as_fpsgame_mode))
  (Default|TookDamage _hud (Variables|Default|GetHealth))
  (Default|PlayHitAnimation _hud)
  (Class|BHCharacterPlayer|ApplyCameraShake "/Game/Blueprints/FX/BP_CameraShake.BP_CameraShake_C"))

(event Custom|HeadBob
  (bind _returnvalue (Game|GetPlayerController 0))
  (bind _animbp (Variables|Default|GetAnimBP))
  (if (Variables|/Script/BrotherhoodFPS.BH_AnimInstanceBase|GetIsMoving _animbp)
    (if (Variables|/Script/BrotherhoodFPS.BH_AnimInstanceBase|GetIsSprinting _animbp)
      (Game|Feedback|ClientStartCameraShake _returnvalue "/Game/Blueprints/FX/Sprint.Sprint_C" 1.0 "CameraLocal" "0, 0, 0")
      (else
        (Game|Feedback|ClientStartCameraShake _returnvalue "/Game/Blueprints/FX/Walk.Walk_C" 1.0 "CameraLocal" "0, 0, 0")))
    (else
      (Game|Feedback|ClientStartCameraShake _returnvalue "/Game/Blueprints/FX/Idle.Idle_C" 1.0 "CameraLocal" "0, 0, 0"))))

(event EventBeginPlay
  (bind _asfpsgame_mode (Utilities|Casting|CastToFPSGameMode (Game|GetGameMode)))
  (bind _output_get (Variables|Default|SetAs%20FPSGame%20Mode _asfpsgame_mode))
  (Default|TookDamage (Variables|/Game/Blueprints/Game/FPSGameMode.FPSGameMode_C|GetHUD _output_get) (Variables|Default|GetHealth))
  (Default|UpdatePlayerStatParams _output_get))

(event Collision|EventActorBeginOverlap
  (params (OtherActor :type Actor%20Object%20Reference)))

(event EventTick
  (params (DeltaSeconds :type Float%20%28single-precision%29))
  (if (not (Variables|/Script/BrotherhoodFPS.BH_AnimInstanceBase|GetIsAiming (Variables|Default|GetAnimBP)))
    (CallFunction|HeadBob)))

(event EventUpdatePlayerParamStats
  (params (bullet :type Integer) (cartridge :type Integer) (wasHit :type Integer))
  (Default|UpdatePlayerStatParams (Variables|Default|GetAs%20FPSGame%20Mode) cartridge bullet wasHit))

(event EventCheckPlayerIsDead
  (Development|PrintString "Checking if Player Is Dead")
  (CallFunction|UpdateBloodAnimation)
  (if (<= (Variables|Default|GetHealth) 0.0)
    (Default|PlayerDied (Variables|Default|GetAs%20FPSGame%20Mode))))

(fn ConstructionScript
  (Transformation|AttachComponentToComponent (Variables|Default|GetGunComponent) (Variables|Character|GetMesh) "GripPoint" "SnapToTarget" "SnapToTarget" "SnapToTarget" true))
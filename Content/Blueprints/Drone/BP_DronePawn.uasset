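; Enemy drone pawn that patrols linked PatrolPoints, then turns rage-colored and chases the player when they enter its detection sphere or damage it.
; AI move nodes drive movement, while Tick smoothly rotates it toward its current goal.
; Touching the player with its explosion sphere deals damage and detonates it.
; Losing all health passes the final hit's damage to BP_Core, then explodes it with effects and notifies FPSGameMode.
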(event OnComponentBeginOverlap(Sphere)
  (params (OverlappedComponent :type Primitive%20Component%20Object%20Reference) (OtherActor :type Actor%20Object%20Reference) (OtherComp :type Primitive%20Component%20Object%20Reference) (OtherBodyIndex :type Integer) (bFromSweep :type Boolean) (SweepResult :type Hit%20Result%20Structure%20%28by%20ref%29))
  (bind _asbp_player (Utilities|Casting|CastToBP_Player OtherActor))
  (CallFunction|ChangeDroneColor true)
  (CallFunction|MovetoGoalTarget _asbp_player))

(event OnComponentBeginOverlap(ExplosionSphere)
  (params (OverlappedComponent :type Primitive%20Component%20Object%20Reference) (OtherActor :type Actor%20Object%20Reference) (OtherComp :type Primitive%20Component%20Object%20Reference) (OtherBodyIndex :type Integer) (bFromSweep :type Boolean) (SweepResult :type Hit%20Result%20Structure%20%28by%20ref%29))
  (Development|PrintString (Utilities|GetDisplayName OtherActor))
  (bind _asbp_player (Utilities|Casting|CastToBP_Player OtherActor)
    (:then
      (Game|Damage|ApplyDamage _asbp_player (Variables|Default|GetDamage) 0 self)
      (CallFunction|Explode))
    (:CastFailed
      (Development|PrintString "cAST FAILED"))))

(event Custom|OnTakeAnyDamage_Event
  (params (DamagedActor :type Actor%20Object%20Reference) (Damage :type Float%20%28single-precision%29) (DamageType :type Damage%20Type%20Object%20Reference) (InstigatedBy :type Controller%20Object%20Reference) (DamageCauser :type Actor%20Object%20Reference))
  (Development|PrintString "Hit")
  (bind _output_get (Variables|Default|SetHealth (- (Variables|Default|GetHealth) Damage)))
  (if (<= _output_get 0.0)
    (bind _returnvalue (Actor|GetActorOfClass "/Game/Blueprints/Props/BP_Core.BP_Core_C"))
    (Game|Damage|ApplyDamage _returnvalue Damage 0 DamageCauser)
    (CallFunction|Explode)
    (else
      (bind _asbp_player (Utilities|Casting|CastToBP_Player DamageCauser))
      (CallFunction|ChangeDroneColor true)
      (CallFunction|MovetoGoalTarget _asbp_player))))

(event Custom|MoveToGoalTarget
  (params (NewGoalTarget :type Actor%20Object%20Reference))
  (bind _output_get (Variables|Default|SetGoal%20Actor NewGoalTarget))
  (AI|AIMoveTo self "0, 0, 0" _output_get 5.0 false))

(event EventBeginPlay
  (EventDispatchers|AssignOnTakeAnyDamage (delegate Custom|OnTakeAnyDamage_Event))
  (Utilities|Patrol))

(event EventTick
  (params (DeltaSeconds :type Float%20%28single-precision%29))
  (bind _goal_actor (Variables|Default|GetGoal%20Actor))
  (Utilities|IsValid _goal_actor
    (:Is%20Valid
      (Transformation|SetActorRotation (Math|Interpolation|RInterpTo (Transformation|GetActorRotation) (Math|Rotator|FindLookatRotation (Transformation|GetActorLocation) (Transformation|GetActorLocation _goal_actor)) DeltaSeconds 5.0)))))

(fn ConstructionScript
  (|CallParentFunction)
  (bind _returnvalue (Rendering|Material|CreateDynamicMaterialInstance (Rendering|Material|GetMaterial (Variables|Default|GetDroneMesh) 0) "None" "None" :!class /Script/Engine.KismetMaterialLibrary))
  (bind _output_get (Variables|Default|SetDynamicDroneMaterial _returnvalue))
  (Rendering|Material|SetMaterial (Variables|Default|GetDroneMesh) 0 _output_get))

(fn Explode
  (bind _returnvalue (Transformation|GetActorLocation))
  (Effects|SpawnEmitteratLocation (Variables|Default|GetExplodeFX) _returnvalue (Transformation|GetActorRotation))
  (Audio|PlaySoundatLocation (Variables|Default|GetExplosionSound) _returnvalue "0, 0, 0" 1.0 1.0 0.0 0 0 0 0)
  (bind _asfpsgame_mode (Utilities|Casting|CastToFPSGameMode (Game|GetGameMode)))
  (Default|DroneDied _asfpsgame_mode)
  (Actor|DestroyActor))

(fn ChangeDroneColor
  (params (IsInRageMode :type Boolean))
  (if IsInRageMode
    (Rendering|Material|SetVectorParameterValue (Variables|Default|GetDynamicDroneMaterial) "TeamColor" (Variables|Default|GetRageColor) :!class /Script/Engine.MaterialInstanceDynamic)
    (else
      (Rendering|Material|SetVectorParameterValue (Variables|Default|GetDynamicDroneMaterial) "TeamColor" (Variables|Default|GetCoolColor) :!class /Script/Engine.MaterialInstanceDynamic))))
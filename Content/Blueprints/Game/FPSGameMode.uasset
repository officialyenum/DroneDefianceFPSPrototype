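; Game mode for a timed FPS drone-hunting mission, running warm-up, play and win, death or timeout states.
; Tick drives the warm-up countdown, which unlocks input and starts timed control hints, then the game timer.
; Drone deaths update the HUD and quests, leading to the core objective or victory.
; It also tracks player stats, handles pausing, and routes every ending to the WinnerHUD widget.
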(event Custom|StartTutorial
  (Utilities|FlowControl|Delay 2.0)
  (CallFunction|UpdateTutorial "To Aim" "Hold" "/Game/Assets/UI/Inputs/mouse_right.mouse_right")
  (Utilities|FlowControl|Delay 3.0)
  (CallFunction|UpdateTutorial "To Shoot" "Press" "/Game/Assets/UI/Inputs/mouse_left.mouse_left")
  (Utilities|FlowControl|Delay 3.0)
  (CallFunction|UpdateTutorial "To Turn and Look Up" "Move" "/Game/Assets/UI/Inputs/mouse_move.mouse_move")
  (Utilities|FlowControl|Delay 3.0)
  (CallFunction|UpdateTutorial "To Sprint" "Hold" "/Game/Assets/UI/Inputs/keyboard_shift.keyboard_shift")
  (Utilities|FlowControl|Delay 3.0)
  (CallFunction|UpdateTutorial "To Quit " "Press" "/Game/Assets/UI/Inputs/keyboard_escape.keyboard_escape")
  (Utilities|FlowControl|Delay 3.0)
  (CallFunction|UpdateTutorial "To Show Quest" "Press" "/Game/Assets/UI/Inputs/keyboard_q.keyboard_q"))

(event Custom|UpdateTutorial
  (params (ActionT :type Text) (ActionTType :type Text) (Action%20Image :type Object%20Object%20Reference))
  (bind _hud (Variables|Default|GetHUD))
  (bind _wb_controlassistant (Variables|/Game/Blueprints/UI/HUD/WB_CharacterHUD.WB_CharacterHUD_C|GetWB_ControlAssistant _hud))
  (Widget|SetVisibility _wb_controlassistant "Visible")
  (Audio|PlaySound2D "/Engine/EditorSounds/Notifications/CompileStart_Cue.CompileStart_Cue" 1.0 1.0 0.0 0 0)
  (Default|UpdateControlData _wb_controlassistant ActionT ActionTType Action%20Image)
  (Utilities|FlowControl|Delay 2.0)
  (Widget|SetVisibility _wb_controlassistant "Hidden"))

(event Custom|UpdateAnnouncement
  (params (AnnouncementText :type Text) (Color :type Linear%20Color%20Structure))
  (Default|CallOnAnnouncementEvent AnnouncementText Color)
  (Utilities|FlowControl|Delay 5.0)
  (Default|CallOnAnnouncementEvent))

(event Custom|EndGame
  (Utilities|FlowControl|Delay 0.4)
  (CallFunction|ShowWinHUD)
  (Game|SetGamePaused true))

(event Custom|ResumeGame
  (params (PauseMenuWidget :type Widget%20Object%20Reference))
  (bind _playercontroller (Variables|Default|GetPlayerController))
  (Game|SetGamePaused false)
  (Widget|RemovefromParent PauseMenuWidget)
  (Input|SetInputModeGameOnly (Variables|Default|GetPlayerController) false)
  (Variables|/Script/Engine.PlayerController|SetbShowMouseCursor _playercontroller false)
  (Variables|/Script/Engine.PlayerController|SetbEnableClickEvents _playercontroller false)
  (Variables|/Script/Engine.PlayerController|SetbEnableMouseOverEvents _playercontroller false))

(event Custom|PauseGame
  (bind _playercontroller (Variables|Default|GetPlayerController))
  (Game|SetGamePaused true)
  (bind _returnvalue (UserInterface|CreateWidget "/Game/Blueprints/UI/HUD/WB_PauseMenu.WB_PauseMenu_C" _playercontroller))
  (UserInterface|Viewport|AddtoViewport _returnvalue 0)
  (Input|SetInputModeGameandUI _playercontroller _returnvalue "LockAlways" false false)
  (Variables|/Script/Engine.PlayerController|SetbShowMouseCursor _playercontroller true)
  (Variables|/Script/Engine.PlayerController|SetbEnableClickEvents _playercontroller true)
  (Variables|/Script/Engine.PlayerController|SetbEnableMouseOverEvents _playercontroller true))

(event Custom|ShowCharacterHUD
  (UserInterface|Viewport|AddtoViewport (Variables|Default|GetHUD) 0))

(event Custom|ShowWinHUD
  (bind _playercontroller (Variables|Default|GetPlayerController))
  (Game|SetGamePaused true)
  (bind _returnvalue (UserInterface|CreateWidget "/Game/Blueprints/UI/HUD/WB_WinnerHUD.WB_WinnerHUD_C" _playercontroller))
  (UserInterface|Viewport|AddtoViewport _returnvalue 0)
  (Input|SetInputModeGameandUI _playercontroller _returnvalue "LockAlways" true false)
  (Variables|/Script/Engine.PlayerController|SetbShowMouseCursor _playercontroller true)
  (Variables|/Script/Engine.PlayerController|SetbEnableClickEvents _playercontroller true)
  (Variables|/Script/Engine.PlayerController|SetbEnableMouseOverEvents _playercontroller true))

(event EventBeginPlay
  (Utilities|FlowControl|Sequence
    (:then_0
      ;[1 1 1] Setup Controller
      (bind _asbp_player_controller (Utilities|Casting|CastToBP_PlayerController (Game|GetPlayerController 0)))
      (bind _output_get (Variables|Default|SetPlayerController _asbp_player_controller))
      (Input|SetInputModeGameOnly _output_get false))
    (:then_1
      ;[1 1 1] HUD UI Setup
      (bind _returnvalue (UserInterface|CreateWidget "/Game/Blueprints/UI/HUD/WB_CharacterHUD.WB_CharacterHUD_C" (Variables|Default|GetPlayerController)))
      (Variables|Default|SetHUD _returnvalue)
      (CallFunction|ShowCharacterHUD)
      (Default|CallOnAnnouncementEvent "Get Ready !!!" "(R=1.000000,G=1.000000,B=1.000000,A=1.000000)")
      (bind _format_time (CallFunction|TimeRemainingFormat))
      (Default|CallOnTimeUpdateEvent _format_time "(R=1.000000,G=1.000000,B=1.000000,A=1.000000)"))
    (:then_2
      ;[1 1 1] Drones Init
      (bind _outactors (Actor|GetAllActorsOfClass "/Game/Blueprints/Drone/BP_DronePawn.BP_DronePawn_C"))
      (Variables|Default|SetNoOfDrones (Utilities|Array|Length _outactors))
      (CallFunction|UpdateDrones))
    (:then_3
      ;[1 1 1] Disable Player Input
      (CallFunction|DisablePlayerInput))))

(event EventTick
  (params (DeltaSeconds :type Float%20%28single-precision%29))
  (switch Utilities|FlowControl|Switch|SwitchonE_SessionState (Variables|Default|GetSessionState)
    (:NewEnumerator0
      (CallFunction|UpdateWarmupTimer))
    (:NewEnumerator1
      (CallFunction|UpdateGameTimer DeltaSeconds))))

(fn ConstructionScript)

(fn UpdateDrones
  (Rendering|Components|TextRender|SetText (Variables|/Game/Blueprints/UI/HUD/WB_CharacterHUD.WB_CharacterHUD_C|GetDroneText (Variables|Default|GetHUD)) (Utilities|Text|ToText(Integer) (Variables|Default|GetNoOfDrones))))

(fn DroneDied
  (bind _result (Math|Integer|DecrementInt (Variables|Default|GetNoOfDrones))
    (:%20%20
      (CallFunction|UpdateDrones)
      (if (<= _result 0)
        (CallFunction|UpdateQuest (Utilities|String|MakeLiteralString "Eliminate All Drones in Area"))
        (bind _returnvalue (Actor|GetActorOfClass "/Game/Blueprints/Props/BP_Core.BP_Core_C"))
        (Utilities|IsValid _returnvalue
          (:Is%20Valid
            (CallFunction|UpdateAnnouncement "Find & Destroy Drone Core" "(R=0.000000,G=1.000000,B=0.106813,A=1.000000)"))
          (:Is%20Not%20Valid
            (CallFunction|UpdateQuest (Utilities|String|MakeLiteralString "Destroy Vorons Shield  Core"))
            (CallFunction|PlayerWon)))))))

(fn UpdateWarmupTimer
  (bind _returnvalue (Utilities|Time|GetGameTimeinSeconds))
  (bind _warmuptime (Variables|Default|GetWarmUpTime))
  (bind _returnvalue_2 (- _warmuptime _returnvalue))
  (bind _returnvalue_3 (Class|KismetMathLibrary|FCeil64 _returnvalue_2))
  (Rendering|Components|TextRender|SetText (Variables|/Game/Blueprints/UI/HUD/WB_CharacterHUD.WB_CharacterHUD_C|GetWarmUpText (Variables|Default|GetHUD)) (Utilities|Text|ToText(String) _returnvalue_3))
  (if (<= _returnvalue_3 0)
    (CallFunction|StartGame)))

(fn DisablePlayerInput
  (bind _asbp_player (Utilities|Casting|CastToBP_Player (Game|Player|GetPlayerPawn 0)))
  (Variables|/Script/BrotherhoodFPS.BH_CharacterBase|SetFireButtonPressed _asbp_player false)
  (bind _asbp_player_controller (Utilities|Casting|CastToBP_PlayerController (Game|GetPlayerController 0)))
  (Input|DisableInput _asbp_player_controller _asbp_player_controller))

(fn EnablePlayerInput
  (bind _returnvalue (Game|Player|GetPlayerPawn 0))
  (bind _asbp_player (Utilities|Casting|CastToBP_Player _returnvalue))
  (Variables|/Script/BrotherhoodFPS.BH_CharacterBase|SetFireButtonPressed _asbp_player true)
  (Input|EnableInput _returnvalue 0))

(fn StartGame
  (bind _hud (Variables|Default|GetHUD))
  (Variables|Default|SetSessionState "NewEnumerator1")
  (bind _asbp_player_controller (Utilities|Casting|CastToBP_PlayerController (Pawn|GetController (Game|Player|GetPlayerPawn 0))))
  (Input|EnableInput _asbp_player_controller _asbp_player_controller)
  (Rendering|Components|TextRender|SetText (Variables|/Game/Blueprints/UI/HUD/WB_CharacterHUD.WB_CharacterHUD_C|GetWarmUpText _hud) "")
  (Rendering|Components|TextRender|SetText (Variables|/Game/Blueprints/UI/HUD/WB_CharacterHUD.WB_CharacterHUD_C|GetAnnouncementText _hud) "")
  (CallFunction|StartTutorial))

(fn UpdateGameTimer
  (params (Delta%20Time :type Float%20%28double-precision%29))
  (bind _output_get (Variables|Default|SetTimeRemaining (- (Variables|Default|GetTimeRemaining) Delta%20Time)))
  (Variables|Default|SetPlayerState (Utilities|Struct|MakeS_PlayerStat (.rank (Variables|Default|GetPlayerState)) (Math|Float|Truncate _output_get) (.cartridgeused (Variables|Default|GetPlayerState)) (.bulletsshot (Variables|Default|GetPlayerState)) (.damagetakencount (Variables|Default|GetPlayerState))))
  (bind _format_time (CallFunction|TimeRemainingFormat))
  (if (<= _output_get 15.0)
    (Default|CallOnTimeUpdateEvent _format_time "(R=1.000000,G=0.043458,B=0.000000,A=1.000000)")
    (if (<= _output_get 0.0)
      (CallFunction|OutOfTime))
    (else
      (Default|CallOnTimeUpdateEvent _format_time "(R=1.000000,G=1.000000,B=1.000000,A=1.000000)"))))

(fn OutOfTime
  (Variables|Default|SetSessionState "NewEnumerator2")
  (Default|CallOnTimeUpdateEvent "00:00" "(R=1.000000,G=0.043458,B=0.000000,A=1.000000)")
  (Default|CallOnAnnouncementEvent "Out Of Time" "(R=1.000000,G=0.043458,B=0.000000,A=1.000000)")
  (CallFunction|DisablePlayerInput)
  (CallFunction|EndGame))

(fn TimeRemainingFormat
  (bind _timeremaining (Variables|Default|GetTimeRemaining))
  (bind _returnvalue (/ _timeremaining 6e+01))
  (bind _returnvalue_2 (Class|KismetMathLibrary|FFloor64 _returnvalue))
  (return (Utilities|Text|FormatText "{Minutes}:{Seconds}" (Utilities|Text|ToText(String) _returnvalue_2) (Utilities|Text|ToText(Float) (- (Variables|Default|GetTimeRemaining) (* _returnvalue_2 60)) "HalfToEven" false true 2 2 0 0))))

(fn PlayerWon
  (Variables|Default|SetSessionState "NewEnumerator4")
  (CallFunction|UpdateAnnouncement "Mission Accomplished !!" "(R=0.000000,G=1.000000,B=0.106813,A=1.000000)")
  (Audio|PlaySound2D "/Game/Assets/Sounds/Voice/DroneDefiance-MissionAccomplished_Cue.DroneDefiance-MissionAccomplished_Cue" 1.2 1.0 0.0 0 0)
  (CallFunction|DisablePlayerInput)
  (CallFunction|EndGame))

(fn PlayerDied
  (Variables|Default|SetSessionState "NewEnumerator3")
  (CallFunction|UpdateAnnouncement "You Died !!!" "(R=1.000000,G=0.043458,B=0.000000,A=1.000000)")
  (CallFunction|DisablePlayerInput)
  (CallFunction|EndGame))

(fn UpdateQuest
  (params (Key :type String%20%28by%20ref%29))
  (bind _hud (Variables|Default|GetHUD))
  (Utilities|Map|Add (Variables|Default|GetQuestList) Key true)
  (Default|UpdateQuestList (Variables|/Game/Blueprints/UI/HUD/WB_CharacterHUD.WB_CharacterHUD_C|GetWB_QuestListView _hud) self)
  (Default|ToggleQuestWidget _hud)
  (return))

(fn UpdatePlayerStatParams
  (params (CartridgeUsed :type Integer) (BulletsShot :type Integer) (DamageTakenCount :type Integer))
  (bind _output_get (Variables|Default|SetPlayerState (Utilities|Struct|MakeS_PlayerStat (.rank (Variables|Default|GetPlayerState)) (Math|Float|Truncate (Variables|Default|GetTimeRemaining)) (+ CartridgeUsed (.cartridgeused (Variables|Default|GetPlayerState))) (+ BulletsShot (.bulletsshot (Variables|Default|GetPlayerState))) (+ DamageTakenCount (.damagetakencount (Variables|Default|GetPlayerState))))))
  (Default|CallOnPlayerStateUpdateEvent _output_get))